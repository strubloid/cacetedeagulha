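; BP_Sword is a thrown sword projectile that damages enemies or embeds in surfaces as a platform for the player.
; Overlapping a BP_Enemy passes ThrowDamage through ReceiveAttack and destroys the sword.
; On a Box hit, it switches to a non-looping embedded flipbook and shifts the sprite to the EmbededPosition offset.
; The box then blocks the Pawn channel and is resized so the player can stand on it.
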(event OnComponentHit(Box)
  (params (HitComponent :type Primitive%20Component%20Object%20Reference) (OtherActor :type Actor%20Object%20Reference) (OtherComp :type Primitive%20Component%20Object%20Reference) (NormalImpulse :type Vector :default "0, 0, 0") (Hit :type Hit%20Result%20Structure%20%28by%20ref%29))
  ;[1 0.2889 0.3487] When we hit something, we change the sword flipbook
  (Sprite|SetFlipbook (Variables|Default|GetWeaponFlipbook) "/Game/PaperAssets/Sword/Captain__Sword_Embedded.Captain__Sword_Embedded")
  ;[1 0.8446 0.3222] Set the flipbook to not loop
  (Components|Timeline|SetLooping (Variables|Default|GetWeaponFlipbook) false)
  ;[0.1622 0.28 1 1 14] Here we are getting the relative location an setting it, so when we hit the target, will move some position bacwards to fit on the wall the sprite
  (Transformation|SetRelativeLocation (Variables|Default|GetWeaponFlipbook) (Variables|/Script/Engine.SceneComponent|GetRelativeLocation (Variables|Default|GetEmbededPosition)) false false)
  ;[1 1 1 1 14] After we finish hit the target, we want the sword to stick to it, so needs to block colision to the player, so they can hop in
  (Collision|SetCollisionResponsetoChannel (Variables|Default|GetBox) "ECC_Pawn" "ECR_Block")
  ;[0.1571 0.4382 1 1 14] Changing the z dimension so the player isnt flying on the top of the sword, instead of being correct set, this is the fix for it.
  (Components|Box|SetBoxExtent (Variables|Default|GetBox) "0.000000,20.000000,10.000000" true))

(event OnComponentBeginOverlap(Box)
  (params (OverlappedComponent :type Primitive%20Component%20Object%20Reference) (OtherActor :type Actor%20Object%20Reference) (OtherComp :type Primitive%20Component%20Object%20Reference) (OtherBodyIndex :type Integer) (bFromSweep :type Boolean) (SweepResult :type Hit%20Result%20Structure%20%28by%20ref%29))
  ;[1 0.06771 0.06771] Set the sword throw damage
  (bind _asbp_enemy (Utilities|Casting|CastToBP_Enemy OtherActor))
  (Default|ReceiveAttack _asbp_enemy (Variables|Default|GetThrowDamage))
  (Actor|DestroyActor))

(event EventBeginPlay)

(event Collision|EventActorBeginOverlap
  (params (OtherActor :type Actor%20Object%20Reference)))

(event EventTick
  (params (DeltaSeconds :type Float%20%28single-precision%29)))

(fn ConstructionScript)