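; BP_Ability_Pickup is a pickup that grants its ability type to BP_Player when overlapped.
; The PlayerCheck overlap runs Setup to cache the player and its WID_Player widget, then calls GainAbility, CreateSkill and UpdateWidget.
; CreateSkill and UpdateWidget have no bodies in this file.
; Before destroying itself, the pickup tells each entry in Spawners to spawn a BP_Enemy.
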(event OnComponentBeginOverlap(PlayerCheck)
  (params (OverlappedComponent :type Primitive%20Component%20Object%20Reference) (OtherActor :type Actor%20Object%20Reference) (OtherComp :type Primitive%20Component%20Object%20Reference) (OtherBodyIndex :type Integer) (bFromSweep :type Boolean) (SweepResult :type Hit%20Result%20Structure%20%28by%20ref%29))
  ;[0.1922 1 0.4551 1 14] Setup of the main variables
  (CallFunction|Setup OtherActor)
  ;[1 0.89 0.3345 1 12] We get the ability attached once to the character player
  (Default|GainAbility (Variables|Default|GetBP_Player) (Variables|Default|GetAbilityType))
  ;[1 0.4696 0.5462 1 14] Ask for the ability to build on the character
  (CallFunction|CreateSkill)
  ;[0.4893 0.6217 1 1 14] Ask the Ability to update widget
  (CallFunction|UpdateWidget)
  ;[1 0.7965 0.111] We are going to spawn thing before destroy the object
  (for _array_element (Variables|Default|GetSpawners)
    (Default|SpawnEnemy _array_element "/Game/Blueprints/Characters/Enemies/BP_Enemy.BP_Enemy_C"))
  ;[1 0 0] Finish of the functionality
  (Actor|DestroyActor))

(event EventBeginPlay)

(event Collision|EventActorBeginOverlap
  (params (OtherActor :type Actor%20Object%20Reference)))

(event EventTick
  (params (DeltaSeconds :type Float%20%28single-precision%29)))

(fn ConstructionScript
  (|CallParentFunction))

(fn Setup
  (params (Object :type Object%20Object%20Reference))
  ;[1 0.7479 0.217] Set of the BP_Player
  (bind _asbp_player (Utilities|Casting|CastToBP_Player Object))
  (bind _output_get (Variables|Default|SetBP_Player _asbp_player))
  ;[1 0.444 0.1596 1 14] We are triggering the WID_Player to get the projectile quantity
  (Variables|Default|SetWID_Player (Variables|/Game/Blueprints/Characters/Player/BP_Player.BP_Player_C|GetWID_Player _output_get)))