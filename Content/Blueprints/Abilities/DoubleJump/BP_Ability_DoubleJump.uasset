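; Double jump ability Blueprint that raises the player's maximum jump count when its overlap is processed.
; BeginPlay runs the parent logic, then sets the skill's maximum activation count and its ability type.
; ProcessOverlap calls the parent implementation, then adds JumpIncrementFrom to the player's JumpMaxCount.
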(event EventBeginPlay
  (|CallParentFunction)
  ;[1 1 1] Starting the max count
  (Variables|Default|SetMaxTimesActivateSkill 2)
  (Variables|Default|SetAbilityType "NewEnumerator0"))

(event Collision|EventActorBeginOverlap
  (params (OtherActor :type Actor%20Object%20Reference))
  (|CallParentFunction OtherActor) ; This node is disabled and will not be called.\nDrag off pins to build functionality.
)

(event EventTick
  (params (DeltaSeconds :type Float%20%28single-precision%29))
  (|CallParentFunction DeltaSeconds) ; This node is disabled and will not be called.\nDrag off pins to build functionality.
)

(fn ConstructionScript
  (|CallParentFunction))

(fn ProcessOverlap
  (params (BP_Player :type BP%20Player%20Object%20Reference))
  (|CallParentFunction BP_Player)
  ;[0 1 0.06377] Set of the Ability
  (Variables|/Script/Engine.Character|SetJumpMaxCount (Variables|Default|GetBP_Player) (+ (Variables|/Script/Engine.Character|GetJumpMaxCount (Variables|Default|GetBP_Player)) (Variables|Default|GetJumpIncrementFrom))))