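; BP_Throw_Power is a child Blueprint that grants the player a throw power ability with a limited number of uses.
; BeginPlay sets the ability type and maximum activation count after calling the parent.
; CreateSkill has the player gain that ability and sets its ability count to the maximum.
; UpdateWidget pushes the count to the player widget and appends the ability's enum name to its comma-separated skills text.
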(event EventBeginPlay
  (|CallParentFunction)
  ;[1 1 1] Starting the max count
  (Variables|Default|SetMaxTimesActivateSkill 6)
  (Variables|Default|SetAbilityType "NewEnumerator1"))

(event Collision|EventActorBeginOverlap
  (params (OtherActor :type Actor%20Object%20Reference))
  (|CallParentFunction OtherActor) ; This node is disabled and will not be called.\nDrag off pins to build functionality.
)

(event EventTick
  (params (DeltaSeconds :type Float%20%28single-precision%29))
  (|CallParentFunction DeltaSeconds) ; This node is disabled and will not be called.\nDrag off pins to build functionality.
)

(event EventCreateSkill
  ;[1 0.89 0.3345 1 12] We get the ability attached once to the character player
  (Default|GainAbility (Variables|Default|GetBP_Player) (Variables|Default|GetAbilityType))
  ;[1 1 1 1 14] Set count for this skill
  (Variables|/Game/Blueprints/Characters/Player/BP_Player.BP_Player_C|SetAbilityCount (Variables|Default|GetBP_Player) (Variables|Default|GetMaxTimesActivateSkill)))

(event EventUpdateWidget
  ;[1 1 1 1 14] Update count into widget
  (Default|UpdateProjectilesEvent (Variables|Default|GetWID_Player) (Variables|Default|GetMaxTimesActivateSkill))
  ;[1 1 1 1 14] Skill text
  (Default|UpdateSkillsEvent (Variables|Default|GetWID_Player) (Utilities|String|Append (Utilities|String|ToString(Text) (Variables|/Script/UMG.TextBlock|GetText (Variables|/Game/Blueprints/GameState/Widgets/Player/WID_Player.WID_Player_C|GetWID_Skills (Variables|Default|GetWID_Player)))) "," (Utilities|String|EnumtoString (Variables|Default|GetAbilityType self)))))

(fn ConstructionScript
  (|CallParentFunction))