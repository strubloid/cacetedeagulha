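; Heal ability actor that restores the player's health by HealQuantity.
; On BeginPlay it sets its ability type and appends the truncated heal amount to its Ability text.
; CreateSkill calls IncreaseHealth on the player's character component, and UpdateWidget pushes current health to the player widget and refreshes the health percentage widget.
; Its own PlayerCheck overlap event is empty.
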(event OnComponentBeginOverlap(PlayerCheck)
  (params (OverlappedComponent :type Primitive%20Component%20Object%20Reference) (OtherActor :type Actor%20Object%20Reference) (OtherComp :type Primitive%20Component%20Object%20Reference) (OtherBodyIndex :type Integer) (bFromSweep :type Boolean) (SweepResult :type Hit%20Result%20Structure%20%28by%20ref%29)))

(event EventBeginPlay
  (|CallParentFunction)
  (Variables|Default|SetAbilityType "NewEnumerator2")
  ;[0.211 0.09678 0.526 1 14] Set of the text of the life based in the heal quantity
  (Rendering|Components|TextRender|SetText (Variables|Default|GetAbility) (Utilities|Text|ToText(String) (Utilities|String|Append (Utilities|String|ToString(Text) (Variables|/Script/Engine.TextRenderComponent|GetText (Variables|Default|GetAbility))) " " (Utilities|String|ToString(Integer) (Math|Float|Truncate (Variables|Default|GetHealQuantity)))))))

(event Collision|EventActorBeginOverlap
  (params (OtherActor :type Actor%20Object%20Reference))
  (|CallParentFunction OtherActor) ; This node is disabled and will not be called.\nDrag off pins to build functionality.
)

(event EventTick
  (params (DeltaSeconds :type Float%20%28single-precision%29))
  (|CallParentFunction DeltaSeconds) ; This node is disabled and will not be called.\nDrag off pins to build functionality.
)

(event EventCreateSkill
  ;[0 1 0.06377] Set of the Ability
  (Default|IncreaseHealth (Variables|/Game/Blueprints/Characters/Player/BP_Player.BP_Player_C|GetBPC_Character (Variables|Default|GetBP_Player)) (Variables|Default|GetHealQuantity)))

(event EventUpdateWidget
  ;[0.2354 0.3474 0.6302 1 14] Update WID_Player
  (Default|UpdateLifeEvent (Variables|Default|GetWID_Player) (Variables|/Game/Blueprints/Characters/BPC_Character.BPC_Character_C|GetCurrentHealth (Variables|Default|GetBPC_Character)))
  ;[0.2442 0.0449 0.2448 1 14] Update on the widget
  (Default|SetWidgetHealthPercentage (Variables|Default|GetBP_Player) (Variables|Default|GetWID_Health)))

(fn ConstructionScript
  (|CallParentFunction))