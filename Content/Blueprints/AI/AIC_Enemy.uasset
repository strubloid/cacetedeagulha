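; AI controller for enemy characters that runs the BT_Enemy behavior tree on the BB_Enemy blackboard.
; On possess it binds to the character's stunned-state change and mirrors it to the blackboard, while SetAttackTarget stores the target there and locally.
; Each tick it sets the focal point toward the target along the X axis only, or straight ahead when there is no target or the character cannot act.
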(event Custom|OnStunStateChanged
  (params (IsStunned :type Boolean))
  ;[0.4549 0.7631 1] Triggers the set of the value
  (AI|Components|Blackboard|SetValueasBool (Variables|Default|GetBlackboard) (Variables|Default|GetIsStunnedKey) IsStunned))

(event EventBeginPlay
  ;[0.3702 0.4144 1] This sets the blackboard of the AI
  (Class|AIController|UseBlackboard "/Game/Blueprints/AI/BB_Enemy.BB_Enemy")
  ;[1 1 1 1 14] This is to start the behaviour tree, so will be doing the actions that you prorgam over there
  (AI|RunBehaviorTree "/Game/Blueprints/AI/BT_Enemy.BT_Enemy"))

(event EventTick
  (params (DeltaSeconds :type Float%20%28single-precision%29))
  (CallFunction|SetFocusDirection))

(event EventPossess
  (params (PossessedPawn :type Pawn%20Object%20Reference))
  ;[1 1 1] binds the stunned state change event
  (bind _asbp_character (Utilities|Casting|CastToBP_Character PossessedPawn))
  (bind _output_get (Variables|Default|SetActionChar _asbp_character))
  (EventDispatchers|BindEventtoStunnedStateChanged _output_get (delegate Custom|OnStunStateChanged)))

(fn ConstructionScript)

(fn SetAttackTarget
  (params (AttackTarget :type BP%20Player%20Object%20Reference))
  ;[1 0.8333 0.4177 1 15] Sets the target, key and later saves the reference
  (AI|Components|Blackboard|SetValueasObject (Variables|Default|GetBlackboard) (Variables|Default|GetAttackTargetKey) AttackTarget)
  (Variables|Default|SetAttackTarget AttackTarget))

(fn SetFocusDirection
  ;[0.3944 0.5036 1] Checking if exist a target
  (Utilities|IsValid (Variables|Default|GetAttackTarget)
    (:Is%20Valid
      ;[1 0.9307 0.4125 1 15] We arent allowing to change the position while attacaking or stunned
      (if (Default|CanAct (Variables|Default|GetActionChar))
        ;[0.3352 0.3954 1] Rotate Action calulation
        (AI|SetFocalPoint (+ (Transformation|GetActorLocation (Variables|Default|GetActionChar)) (Math|Vector|MakeVector (.x (Math|Vector|GetForwardVector (Math|Rotator|FindLookatRotation (Transformation|GetActorLocation (Variables|Default|GetActionChar)) (Transformation|GetActorLocation (Variables|Default|GetAttackTarget))))) 0.0 0.0)))
        (else
          ;[1 0.151 0.151] Getting a small value in front of our face and setting it.
          (CallFunction|GetDefaultCharacterPosition))))
    (:Is%20Not%20Valid
      ;[1 0.1042 0.1042] Getting a small value in front of our face and setting it.
      (CallFunction|GetDefaultCharacterPosition))))

(fn GetDefaultCharacterPosition
  (bind _actionchar (Variables|Default|GetActionChar))
  (AI|SetFocalPoint (+ (Transformation|GetActorLocation _actionchar) (Transformation|GetActorForwardVector _actionchar))))