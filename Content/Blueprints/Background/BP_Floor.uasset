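; BP_Floor is a background floor actor that builds a run of meshes along a spline.
; The construction script divides the spline length by MeshLength, truncates it, and adds one spline mesh component per whole segment, leaving any remainder uncovered.
; Each segment takes local positions and tangents from its distances along the spline, with tangents clamped to MeshLength to prevent distortion, and attaches to the spline.
; The event graph has no active logic.
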(event EventBeginPlay)

(event Collision|EventActorBeginOverlap
  (params (OtherActor :type Actor%20Object%20Reference)))

(event EventTick
  (params (DeltaSeconds :type Float%20%28single-precision%29)))

(fn ConstructionScript
  (bind _spline (Variables|Default|GetSpline))
  (bind _meshlength (Variables|Default|GetMeshLength))
  (bind _returnvalue (Spline|GetSplineLength _spline))
  (bind _returnvalue_2 (/ _returnvalue _meshlength))
  (bind _returnvalue_3 (Math|Float|Truncate _returnvalue_2))
  ;[1 0.125 0.125 1 14] Checking ithe value is positive, so we can do something
  (if (> _returnvalue_3 0)
    (for _index (range 0 (- _returnvalue_3 1))
      ;[0.05684 0.2969 0.08964 1 14] We are starting the mesh component here, we fix the positon with start and end. and we are attaching the mesh component to the spline
      (bind _returnvalue_4 (AddComponent|AddSplineMeshComponent false))
      (Variables|Default|SetTarget _returnvalue_4)
      (SplineMesh|SetStartandEnd (Variables|Default|GetTarget) (Spline|GetLocationatDistanceAlongSpline (Variables|Default|GetSpline) (* _index (Variables|Default|GetMeshLength)) "Local") (Math|Vector|ClampVectorSize (Spline|GetTangentatDistanceAlongSpline (Variables|Default|GetSpline) (* _index (Variables|Default|GetMeshLength)) "Local") 1.0 (Variables|Default|GetMeshLength)) (Spline|GetLocationatDistanceAlongSpline (Variables|Default|GetSpline) (* (+ _index 1) (Variables|Default|GetMeshLength)) "Local") (Math|Vector|ClampVectorSize (Spline|GetTangentatDistanceAlongSpline (Variables|Default|GetSpline) (* (+ _index 1) (Variables|Default|GetMeshLength)) "Local") 1.0 (Variables|Default|GetMeshLength)) true :!class /Script/Engine.SplineMeshComponent)
      (Transformation|AttachComponentToComponent (Variables|Default|GetTarget) (Variables|Default|GetSpline) "None" "KeepRelative" "KeepRelative" "KeepRelative" true))))