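; BP_Goal is the stage goal trigger that shows a win message and restarts the game when BP_Player reaches it.
; It creates a WID_Message widget on BeginPlay and adds it to the viewport.
; A player overlap on its Box fires once, shows the win text, waits RestartTimer, hides it, then calls RestartGame on GM_CaceteDeAgulha.
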(event OnComponentBeginOverlap(Box)
  (params (OverlappedComponent :type Primitive%20Component%20Object%20Reference) (OtherActor :type Actor%20Object%20Reference) (OtherComp :type Primitive%20Component%20Object%20Reference) (OtherBodyIndex :type Integer) (bFromSweep :type Boolean) (SweepResult :type Hit%20Result%20Structure%20%28by%20ref%29))
  ;[0.3488 1 0.8629] End of the phase, for now we are restarting to the same, but here you can add the change to another one
  (Utilities|Casting|CastToBP_Player OtherActor)
  (Utilities|FlowControl|DoOnce false
    (:Completed
      (bind _aswid_message (Utilities|Casting|CastToWID_Message (Variables|Default|GetWID_Message)))
      (Default|SetFinishStageMessage _aswid_message "You Win")
      (Default|ShoworHideMessage (Variables|Default|GetWID_Message) "Visible")
      ;[1 0.8518 0.2102 1 14] After Delay We remove the text
      (Utilities|FlowControl|Delay (Variables|Default|GetRestartTimer))
      (Default|ShoworHideMessage (Variables|Default|GetWID_Message) "Hidden")
      ;[1 0 0 1 14] Restart
      (bind _asgm_cacete_de_agulha (Utilities|Casting|CastToGM_CaceteDeAgulha (Game|GetGameMode)))
      (Default|RestartGame _asgm_cacete_de_agulha))))

(event EventBeginPlay
  ;[1 1 1] Creating the widget message for the goal class
  (bind _returnvalue (UserInterface|CreateWidget "/Game/Blueprints/Widgets/WID_Message.WID_Message_C" (Game|GetPlayerController 0)))
  (bind _output_get (Variables|Default|SetWID_Message _returnvalue))
  (UserInterface|Viewport|AddtoViewport _output_get 0))

(event Collision|EventActorBeginOverlap
  (params (OtherActor :type Actor%20Object%20Reference)))

(event EventTick
  (params (DeltaSeconds :type Float%20%28single-precision%29)))

(fn ConstructionScript)