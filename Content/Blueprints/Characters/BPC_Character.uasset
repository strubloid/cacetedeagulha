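; Character component that stores health and stamina and mirrors them on the player's HUD.
; BeginPlay caches player 0 as BP_Player, floors current values at zero and initializes the bars.
; Functions change current or max values, capping gains at max but not clamping losses, and write directly to WIDPlayerUI.
; DecreaseHealth returns true on death, while DecreaseStamina returns whether health remains above zero, ignoring remaining stamina.
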(event EventBeginPlay
  ;[0.1389 0.4531 0.1532 1 14] Set BP_Player
  (bind _asbp_player (Utilities|Casting|CastToBP_Player (Game|GetPlayerCharacter 0)))
  (bind _output_get (Variables|Default|SetBP_Player _asbp_player))
  (Utilities|IsValid _output_get
    (:Is%20Valid
      ;[0.401 0.1539 0.2794 1 14] Making sure we do not have negative numbers
      (if (> (Variables|Stamina|GetCurrentStamina) 0.0)
        _
        (else
          (Variables|Stamina|SetCurrentStamina 0.0)))
      ;[0.1085 0.25 0.06791 1 14] Set of the percent of the stamina on the widget player
      (Utilities|IsValid (Variables|/Game/Blueprints/Characters/Player/BP_Player.BP_Player_C|GetWID_PlayerUI (Variables|Default|GetBP_Player))
        (:Is%20Valid
          (Progress|SetPercent (Variables|/Game/Blueprints/Characters/Player/WID_PlayerUI.WID_PlayerUI_C|GetStamina (Variables|/Game/Blueprints/Characters/Player/BP_Player.BP_Player_C|GetWID_PlayerUI (Variables|Default|GetBP_Player))) (/ (Variables|Stamina|GetCurrentStamina) (Variables|Stamina|GetMaxStamina)))
          ;[0.401 0.1539 0.2794 1 14] Making sure we do not have negative numbers
          (if (> (Variables|Health|GetCurrentHealth) 0.0)
            _
            (else
              (Variables|Health|SetCurrentHealth 0.0)))
          ;[0.1085 0.25 0.06791 1 14] Set of the percent of the health on the widget player
          (Progress|SetPercent (Variables|/Game/Blueprints/Characters/Player/WID_PlayerUI.WID_PlayerUI_C|GetHealth (Variables|/Game/Blueprints/Characters/Player/BP_Player.BP_Player_C|GetWID_PlayerUI (Variables|Default|GetBP_Player))) (/ (Variables|Health|GetCurrentHealth) (Variables|Health|GetMaxHealth)))
          ;[0.4792 0.2163 0.007487 1 14] Update of the widget
          (Rendering|Components|TextRender|SetText (Variables|/Game/Blueprints/Characters/Player/WID_PlayerUI.WID_PlayerUI_C|GetHealthValue (Variables|/Game/Blueprints/Characters/Player/BP_Player.BP_Player_C|GetWID_PlayerUI (Variables|Default|GetBP_Player))) (Utilities|Text|ToText(Float) (Variables|Health|GetCurrentHealth) "HalfToEven")))))))

(event EventTick
  (params (DeltaSeconds :type Float%20%28single-precision%29)))

(fn IncreaseMaxHealth
  (params (Health :type Float%20%28double-precision%29))
  ;[0.07681 0.401 0.04008 1 14] Increasing the size of how much health the character gets
  (Variables|Health|SetMaxHealth (+ Health (Variables|Health|GetMaxHealth)))
  ;[0.1085 0.25 0.06791 1 14] Set of the percent of the health on the widget player
  (Progress|SetPercent (Variables|/Game/Blueprints/Characters/Player/WID_PlayerUI.WID_PlayerUI_C|GetHealth (Variables|/Game/Blueprints/Characters/Player/BP_Player.BP_Player_C|GetWID_PlayerUI (Variables|Default|GetBP_Player))) (/ (Variables|Health|GetCurrentHealth) (Variables|Health|GetMaxHealth)))
  ;[0.4792 0.2163 0.007487 1 14] Update of the widget
  (Rendering|Components|TextRender|SetText (Variables|/Game/Blueprints/Characters/Player/WID_PlayerUI.WID_PlayerUI_C|GetHealthValue (Variables|/Game/Blueprints/Characters/Player/BP_Player.BP_Player_C|GetWID_PlayerUI (Variables|Default|GetBP_Player))) (Utilities|Text|ToText(Float) (Variables|Health|GetCurrentHealth) "HalfToEven")))

(fn DecreaseHealth
  (params (Damage :type Float%20%28double-precision%29))
  ;[0.1318 0.4622 0.5312 1 14] Decrease the health of the character
  (Variables|Health|SetCurrentHealth (- (Variables|Health|GetCurrentHealth) Damage))
  ;[0.1085 0.25 0.06791 1 14] Set of the percent of the health on the widget player
  (Progress|SetPercent (Variables|/Game/Blueprints/Characters/Player/WID_PlayerUI.WID_PlayerUI_C|GetHealth (Variables|/Game/Blueprints/Characters/Player/BP_Player.BP_Player_C|GetWID_PlayerUI (Variables|Default|GetBP_Player))) (/ (Variables|Health|GetCurrentHealth) (Variables|Health|GetMaxHealth)))
  ;[0.4792 0.2163 0.007487 1 14] Update of the widget
  (Rendering|Components|TextRender|SetText (Variables|/Game/Blueprints/Characters/Player/WID_PlayerUI.WID_PlayerUI_C|GetHealthValue (Variables|/Game/Blueprints/Characters/Player/BP_Player.BP_Player_C|GetWID_PlayerUI (Variables|Default|GetBP_Player))) (Utilities|Text|ToText(Float) (Variables|Health|GetCurrentHealth) "HalfToEven"))
  ;[0.3333 0.03125 0.03125] Checking if the player died
  (if (<= (Variables|Health|GetCurrentHealth) 0.0)
    ;[1 0.03646 0.03646 1 14] The player is dead
    (return true)
    (else
      ;[0.07358 0.2188 0.06889 1 14] the character is alive
      (return false))))

(fn DecreaseStamina
  (params (StaminaDown :type Float%20%28double-precision%29))
  ;[1 1 1 1 14] Decreasing the Stamina
  (Variables|Stamina|SetCurrentStamina (- (Variables|Stamina|GetCurrentStamina) StaminaDown))
  ;[0.1085 0.25 0.06791 1 14] Set of the percent of the stamina on the widget player
  (Progress|SetPercent (Variables|/Game/Blueprints/Characters/Player/WID_PlayerUI.WID_PlayerUI_C|GetStamina (Variables|/Game/Blueprints/Characters/Player/BP_Player.BP_Player_C|GetWID_PlayerUI (Variables|Default|GetBP_Player))) (/ (Variables|Stamina|GetCurrentStamina) (Variables|Stamina|GetMaxStamina)))
  ;[0.4792 0.2163 0.007487 1 14] Update of the widget
  (Rendering|Components|TextRender|SetText (Variables|/Game/Blueprints/Characters/Player/WID_PlayerUI.WID_PlayerUI_C|GetStaminaValue (Variables|/Game/Blueprints/Characters/Player/BP_Player.BP_Player_C|GetWID_PlayerUI (Variables|Default|GetBP_Player))) (Utilities|Text|ToText(Float) (Variables|Stamina|GetCurrentStamina) "HalfToEven"))
  ;[1 1 1 1 14] Checking if the character is dead, so we stop it when it is
  (if (<= (Variables|Health|GetCurrentHealth) 0.0)
    ;[0.4531 0.08732 0.08732 1 14] The character is dead, so we can't run
    (return false)
    (else
      ;[0.03667 0.3333 0.04939 1 14] The character is alive, so we can run
      (return true))))

(fn IncreaseMaxStamina
  (params (Stamina :type Float%20%28double-precision%29))
  ;[0.1519 0.3333 0.09819 1 14] Inscrease of the max stamina
  (Variables|Stamina|SetMaxStamina (+ (Variables|Stamina|GetMaxStamina) Stamina))
  ;[0.1085 0.25 0.06791 1 14] Set of the percent of the stamina on the widget player
  (Progress|SetPercent (Variables|/Game/Blueprints/Characters/Player/WID_PlayerUI.WID_PlayerUI_C|GetStamina (Variables|/Game/Blueprints/Characters/Player/BP_Player.BP_Player_C|GetWID_PlayerUI (Variables|Default|GetBP_Player))) (/ (Variables|Stamina|GetCurrentStamina) (Variables|Stamina|GetMaxStamina))))

(fn IncreaseHealth
  (params (HealthToAdd :type Float%20%28double-precision%29))
  ;[0.02168 0.4219 0.02883 1 14] This will regenerate a little of the life
  (Variables|Health|SetCurrentHealth (+ (Variables|Health|GetCurrentHealth) HealthToAdd))
  ;[0.3698 0.3511 0.03325 1 14] Checking if the current health is trespassing the limit of max health
  (if (> (Variables|Health|GetCurrentHealth) (Variables|Health|GetMaxHealth))
    ;[0.5312 0.06917 0.06917 1 14] This is just to fix if is trespassing
    (Variables|Health|SetCurrentHealth (Variables|Health|GetMaxHealth)))
  ;[0.1085 0.25 0.06791 1 14] Set of the percent of the health on the widget player
  (Progress|SetPercent (Variables|/Game/Blueprints/Characters/Player/WID_PlayerUI.WID_PlayerUI_C|GetHealth (Variables|/Game/Blueprints/Characters/Player/BP_Player.BP_Player_C|GetWID_PlayerUI (Variables|Default|GetBP_Player))) (/ (Variables|Health|GetCurrentHealth) (Variables|Health|GetMaxHealth)))
  ;[0.4792 0.2163 0.007487 1 14] Update of the widget
  (Rendering|Components|TextRender|SetText (Variables|/Game/Blueprints/Characters/Player/WID_PlayerUI.WID_PlayerUI_C|GetHealthValue (Variables|/Game/Blueprints/Characters/Player/BP_Player.BP_Player_C|GetWID_PlayerUI (Variables|Default|GetBP_Player))) (Utilities|Text|ToText(Float) (Variables|Health|GetCurrentHealth) "HalfToEven")))

(fn IncraseStamina
  (params (Stamina :type Float%20%28double-precision%29))
  ;[0.1002 0.2448 0.07527 1 14] Adding stamina
  (Variables|Stamina|SetCurrentStamina (+ (Variables|Stamina|GetCurrentStamina) Stamina))
  ;[0.3385 0.04761 0.04761 1 14] Checking if we overload the stamina
  (if (> (Variables|Stamina|GetCurrentStamina) (Variables|Stamina|GetMaxStamina))
    ;[1 1 1 1 14] Fixing when is needed
    (Variables|Stamina|SetCurrentStamina (Variables|Stamina|GetMaxStamina)))
  ;[0.1085 0.25 0.06791 1 14] Set of the percent of the stamina on the widget player
  (Progress|SetPercent (Variables|/Game/Blueprints/Characters/Player/WID_PlayerUI.WID_PlayerUI_C|GetStamina (Variables|/Game/Blueprints/Characters/Player/BP_Player.BP_Player_C|GetWID_PlayerUI (Variables|Default|GetBP_Player))) (/ (Variables|Stamina|GetCurrentStamina) (Variables|Stamina|GetMaxStamina)))
  ;[0.4792 0.2163 0.007487 1 14] Update of the widget
  (Rendering|Components|TextRender|SetText (Variables|/Game/Blueprints/Characters/Player/WID_PlayerUI.WID_PlayerUI_C|GetStaminaValue (Variables|/Game/Blueprints/Characters/Player/BP_Player.BP_Player_C|GetWID_PlayerUI (Variables|Default|GetBP_Player))) (Utilities|Text|ToText(Float) (Variables|Stamina|GetCurrentStamina) "HalfToEven")))