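; Sprite-based combat character with faction-checked melee hits, health, stun and defeat.
; Hitbox overlaps with opposing-faction characters deal fixed damage and briefly freeze both actors through CustomTimeDilation hitstop.
; ReceiveAttack plays a sound, subtracts health, then either jumps to the defeated animation and disables capsule collision, or starts a timed stun.
; During stun a looping timer jitters the sprite horizontally, and ClearStun stops it and restores the saved sprite position.
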(event OnComponentBeginOverlap(Hitbox)
  (params (OverlappedComponent :type Primitive%20Component%20Object%20Reference) (OtherActor :type Actor%20Object%20Reference) (OtherComp :type Primitive%20Component%20Object%20Reference) (OtherBodyIndex :type Integer) (bFromSweep :type Boolean) (SweepResult :type Hit%20Result%20Structure%20%28by%20ref%29))
  ;[1 1 1 1 12] we cast to enemies, so we are not hitting ourselves
  (bind _asbp_character (Utilities|Casting|CastToBP_Character OtherActor))
  ;[1 0.9531 0.4922 1 13] Checking if factions are different, otherwise you can hit yourself
  (if (!= (Variables|Default|GetFaction) (Variables|BP_Character_C|GetFaction _asbp_character))
    (CallFunction|ReceiveAttack _asbp_character 25.0)
    ;[0.7213 1 0.6236 1 14] Calling the hitstop on the character
    (CallFunction|HitStopSequence _asbp_character 0.1)
    ;[1 0.2031 0.2031 1 14] we are applying to the enemy here
    (CallFunction|HitStopSequence 0.1)))

(event Custom|HitStopSequence
  (params (Duration :type Float%20%28single-precision%29))
  ;[0.2746 0.3358 1] freezes actor in time
  (Variables|Default|SetCustomTimeDilation 0.0)
  (Utilities|FlowControl|RetriggerableDelay Duration)
  ;[0.5068 1 0.3773] Now is back to normal
  (Variables|Default|SetCustomTimeDilation 1.0))

(event Custom|ShakeSprite
  (bind _sprite_base_location (Variables|Default|GetSprite%20Base%20Location))
  (bind _isa (Utilities|FlowControl|FlipFlop)
    (:A
      _)
    (:B
      _))
  (Transformation|SetRelativeLocation (Variables|Default|GetSprite) (Math|Vector|MakeVector (+ (select _isa (Variables|Default|GetSpriteShakeDistance) (* (Variables|Default|GetSpriteShakeDistance) -1.0)) (.x _sprite_base_location)) (.y _sprite_base_location) (.z _sprite_base_location)) false false))

(event EventBeginPlay
  (CallFunction|SetHitboxCollision false)
  ;[1 0.06244 0.07239 1 12] As we dont need to have a default value, this is the time that we set the max health
  (Variables|Default|SetCurrentHealth (Variables|Default|GetMaxHealth))
  ;[1 1 1] Saving reference of the relative location of the sprite
  (Variables|Default|SetSprite%20Base%20Location (Variables|/Script/Engine.SceneComponent|GetRelativeLocation (Variables|Default|GetSprite))))

(event Collision|EventActorBeginOverlap
  (params (OtherActor :type Actor%20Object%20Reference)))

(event EventTick
  (params (DeltaSeconds :type Float%20%28single-precision%29)))

(fn ConstructionScript)

(fn SetHitboxCollision
  (params (SetActive :type Boolean))
  (if SetActive
    ;[1 1 1] if we have set to active will set the collision to query only
    (Collision|SetCollisionEnabled (Variables|Default|GetHitbox) "QueryOnly")
    (else
      ;[1 1 1] Otherwise will set to no collision
      (Collision|SetCollisionEnabled (Variables|Default|GetHitbox) "NoCollision"))))

(fn ReceiveAttack
  (params (Damage :type Float%20%28double-precision%29))
  ;[0.03881 0.2969 0.09915 1 14] Checking if the character is defeated, so we wouldnt be doing killings over a dead body
  (if (not (Variables|Default|GetIsDefeated))
    ;[1 0.01663 0.613] Play hit sound
    (Audio|PlaySoundatLocation "/Game/Sound/S_Hit_Cue.S_Hit_Cue" (Transformation|GetActorLocation) "0, 0, 0" 1.0 1.0 0.0 0 0 0 0)
    ;[1 0.1534 0.1136] This is the part that we set the damage
    (Variables|Default|SetCurrentHealth (- (Variables|Default|GetCurrentHealth) Damage))
    ;[1 0.7765 0.2187] Check if the health is equal or not to 0
    (if (<= (Variables|Default|GetCurrentHealth) 0.0)
      ;[1 0.125 0.125] Death case, the character is dead.
      (Class|PaperZDAnimInstance|JumptoNode (Class|PaperZDCharacter|GetAnimInstance) "JumpDefeated" "None")
      (Variables|Default|SetIsDefeated true)
      ;[1 1 1] Removing the collision
      (Collision|SetCollisionEnabled (Variables|Default|GetCapsuleComponent) "NoCollision")
      (else
        ;[1 0.7649 0.116] This is the stun case, the character is still alive, but got damage
        ;;[1 0.2795 0.2795 1 13] Set of the condition is being stunned
        (Variables|Default|SetIsStunned true)
        ;;[0.3614 0.3887 1] This will play the animation
        (Class|PaperZDAnimInstance|JumptoNode (Class|PaperZDCharacter|GetAnimInstance) (Variables|Default|GetDefaultStunnedJumpName) "None")
        ;;[0.2032 1 0.2752 1 13] Timer before calling the event, as we want to reset after run
        (Utilities|Time|SetTimerbyEvent (EventDispatchers|CreateEvent :!event ClearStun) (Variables|Default|GetStunLength))
        ;[0.4538 0.4985 1] Triggering the shake when is hit
        (bind _returnvalue (Utilities|Time|SetTimerbyEvent (EventDispatchers|CreateEvent :!event Custom|ShakeSprite) (Variables|Default|GetSpriteShakeFrequency) true))
        (Variables|Default|SetSpriteShakeHandle _returnvalue)))))

(fn ClearStun
  (Variables|Default|SetIsStunned false)
  ;[1 1 1 1 14] This will clear the loop of shake when is hit, at the time stuneed is gone, also the shake
  (Utilities|Time|ClearandInvalidateTimerbyHandle (Variables|Default|GetSpriteShakeHandle))
  ;[0.718 1 0.9801] Setting back the sprite to the base location
  (Transformation|SetRelativeLocation (Variables|Default|GetSprite) (Variables|Default|GetSprite%20Base%20Location) false false))