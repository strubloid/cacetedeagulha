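; BP_Enemy is an enemy character Blueprint that detects the player and reacts to being defeated.
; When a BP_Player overlaps the AggroRange component, it stores that player and passes it to its AIC_Enemy controller as the attack target.
; It binds to the Defeated event on BeginPlay, then moves its Sprite to the DefeatedPosition location and prints a placeholder debug string when that fires.
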(event OnComponentBeginOverlap(AggroRange)
  (params (OverlappedComponent :type Primitive%20Component%20Object%20Reference) (OtherActor :type Actor%20Object%20Reference) (OtherComp :type Primitive%20Component%20Object%20Reference) (OtherBodyIndex :type Integer) (bFromSweep :type Boolean) (SweepResult :type Hit%20Result%20Structure%20%28by%20ref%29))
  ;[0.2602 1 0.2891] This is to check if the enemy can find a player to attack and do it if can find
  (bind _asbp_player (Utilities|Casting|CastToBP_Player OtherActor))
  (Variables|Default|SetPlayer _asbp_player)
  (bind _asaic_enemy (Utilities|Casting|CastToAIC_Enemy (AI|GetAIController self)))
  (Default|SetAttackTarget _asaic_enemy (Variables|Default|GetPlayer)))

(event Custom|OnDefeated
  ;[1 1 1] On Defeated
  (Transformation|SetRelativeLocation (Variables|Default|GetSprite) (Variables|/Script/Engine.SceneComponent|GetRelativeLocation (Variables|Default|GetDefeatedPosition)) false false)
  (Development|PrintString "Hello"))

(event EventBeginPlay
  (|CallParentFunction)
  ;[1 1 1] On Defeated
  (EventDispatchers|BindEventtoDefeated (delegate Custom|OnDefeated)))

(event EventTick
  (params (DeltaSeconds :type Float%20%28single-precision%29)))

(fn ConstructionScript
  (|CallParentFunction))