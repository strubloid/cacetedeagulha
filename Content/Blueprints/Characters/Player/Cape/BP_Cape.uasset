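; BP_Cape is a player character Blueprint that sets the starting stats for the Cape character.
; On BeginPlay it writes current and maximum health and stamina into the BPCCharacter component and sets its own character damage, then calls the parent BeginPlay.
; All other behavior comes from the parent class, as overlap and Tick are disabled stubs and the construction script only calls its parent.
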(event EventBeginPlay
  ;[0.2292 0.01074 0.01074 1 14] Set Component Data
  (Variables|/Game/Blueprints/Characters/BPC_Character.BPC_Character_C|SetCurrentHealth (Variables|Default|GetBPC_Character) 1e+02)
  (Variables|/Game/Blueprints/Characters/BPC_Character.BPC_Character_C|SetMaxHealth (Variables|Default|GetBPC_Character) 1e+02)
  (Variables|/Game/Blueprints/Characters/BPC_Character.BPC_Character_C|SetCurrentStamina (Variables|Default|GetBPC_Character) 1e+02)
  (Variables|/Game/Blueprints/Characters/BPC_Character.BPC_Character_C|SetMaxStamina (Variables|Default|GetBPC_Character) 1e+02)
  ;[0.1891 0.3125 0.1094 1 14] Set player details
  (Variables|Default|SetCharacterDamage 5e+01)
  (|CallParentFunction))

(event Collision|EventActorBeginOverlap
  (params (OtherActor :type Actor%20Object%20Reference))
  (|CallParentFunction OtherActor) ; This node is disabled and will not be called.\nDrag off pins to build functionality.
)

(event EventTick
  (params (DeltaSeconds :type Float%20%28single-precision%29))
  (|CallParentFunction DeltaSeconds) ; This node is disabled and will not be called.\nDrag off pins to build functionality.
)

(fn ConstructionScript
  (|CallParentFunction))