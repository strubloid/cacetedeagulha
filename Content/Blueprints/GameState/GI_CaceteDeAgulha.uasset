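; Game instance for CaceteDeAgulha that manages the persistent high-score scoreboard and creates the message widget on Init.
; LoadScoreboard loads the BP_Scoreboard save from its slot, or creates one if none exists, then re-saves and returns it.
; CreateNewScoreboard writes a fresh scoreboard to that slot without checking for an existing save.
; SaveScoreboard reloads the save, passes the player's total score to SetHighScore and writes it back.
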(event EventInit
  ;[1 0.2552 0.2552 1 14] Widget message load
  (bind _returnvalue (UserInterface|CreateWidget "/Game/Blueprints/GameState/Widgets/Game/Message/WID_Message.WID_Message_C" (Game|GetPlayerController 0)))
  (Variables|Default|SetWID_Message _returnvalue))

(fn LoadScoreboard
  ;[1 0.08854 0.08854 1 14] Check if safe game exist
  (bind _returnvalue (SaveGame|DoesSaveGameExist (Variables|Default|GetScoreboardSlot)))
  (if _returnvalue
    ;[0.6458 0.1013 0.074 1 14] Loads a BP_Scoreboard
    (bind _returnvalue_2 (SaveGame|LoadGamefromSlot (Variables|Default|GetScoreboardSlot)))
    (bind _output_get (Variables|Default|SetScoreboardGameReference _returnvalue_2))
    (bind _asbp_scoreboard (Utilities|Casting|CastToBP_Scoreboard _output_get))
    (bind _output_get_2 (Variables|Default|SetBP_Scoreboard _asbp_scoreboard))
    (SaveGame|SaveGametoSlot _output_get_2 (Variables|Default|GetScoreboardSlot))
    (else
      ;[0.3456 1 0.287 1 14] Create a new BP_Scoreboarad
      (bind _returnvalue_3 (SaveGame|CreateSaveGameObject "/Game/Blueprints/SaveGame/BP_Scoreboard.BP_Scoreboard_C"))
      (bind _output_get_3 (Variables|Default|SetScoreboardGameReference _returnvalue_3))
      (bind _asbp_scoreboard_2 (Utilities|Casting|CastToBP_Scoreboard _output_get_3))
      (bind _output_get_4 (Variables|Default|SetBP_Scoreboard _asbp_scoreboard_2))
      (SaveGame|SaveGametoSlot _output_get_4 (Variables|Default|GetScoreboardSlot))))
  (return (Variables|Default|GetBP_Scoreboard)))

(fn CreateNewScoreboard
  ;[0.3456 1 0.287 1 14] Create a new BP_Scoreboarad
  (bind _returnvalue (SaveGame|CreateSaveGameObject "/Game/Blueprints/SaveGame/BP_Scoreboard.BP_Scoreboard_C"))
  (bind _output_get (Variables|Default|SetScoreboardGameReference _returnvalue))
  ;[0.2093 0.3966 0.4219 1 14] Casting to save this scoreboard
  (bind _asbp_scoreboard (Utilities|Casting|CastToBP_Scoreboard _output_get))
  (bind _output_get_2 (Variables|Default|SetBP_Scoreboard _asbp_scoreboard))
  (SaveGame|SaveGametoSlot _output_get_2 (Variables|Default|GetScoreboardSlot)))

(fn SaveScoreboard
  (params (BP_Player :type BP%20Player%20Object%20Reference))
  (Variables|Default|SetBP%20Player BP_Player)
  ;[0.3456 1 0.287 1 14] Saving the refence of  BP_Scoreboarad
  (bind _returnvalue (SaveGame|LoadGamefromSlot (Variables|Default|GetScoreboardSlot)))
  (bind _output_get (Variables|Default|SetScoreboardGameReference _returnvalue))
  ;[1 0.9385 0.07452 1 14] Loading scoreboard object
  (bind _asbp_scoreboard (Utilities|Casting|CastToBP_Scoreboard _output_get))
  (Variables|Default|SetBP_Scoreboard _asbp_scoreboard)
  ;[0.2093 0.3966 0.4219 1 14] Get Player score and checking if isnt 0
  (bind _returnvalue_2 (Default|GetPlayerTotalScore (Variables|Default|GetBP%20Player)))
  ;[0.5983 0.3485 0.6719 1 14] This is saving to the scoreboard
  (Default|SetHighScore (Variables|Default|GetBP_Scoreboard) _returnvalue_2)
  (SaveGame|SaveGametoSlot (Variables|Default|GetBP_Scoreboard) (Variables|Default|GetScoreboardSlot)))